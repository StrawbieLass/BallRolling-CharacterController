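; BP_LevelEnd is a level exit actor that loads the next numbered level when an overlapping actor has the WinCondition tag.
; On BeginPlay it derives the next level name from the current one by taking the characters after the six-character "Level_" prefix, incrementing that number and rebuilding the name.
; The overlap event then opens that stored level by name.
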(event `self.ReceiveActorBeginOverlap`
  (params (OtherActor :type "Actor Object Reference"))
  (if (`self.ActorHasTag` OtherActor "WinCondition")
    (`GameplayStatics.OpenLevel` (`self.nextLevel`))))

(event `self.ReceiveBeginPlay`
  (bind _returnvalue (`GameplayStatics.GetCurrentLevelName` true))
  (bind _result (`/Engine/EditorBlueprintResources/StandardMacros.IncrementInt` (`KismetStringLibrary.Conv_StringToInt` (`KismetStringLibrary.RightChop` _returnvalue 6)))
    (:`  `
      (set `self.nextLevel` (`KismetStringLibrary.Conv_StringToName` (`KismetStringLibrary.Concat_StrStr` "Level_" (`KismetStringLibrary.Conv_IntToString` _result)))))))

(fn `UserConstructionScript`)