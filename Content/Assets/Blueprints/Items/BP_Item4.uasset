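; BP_Item4 is a pickup item that the player collects by interacting while inside its PickupRadius.
; Overlap caches the third-person character and starts a looping timer that polls its interact flag while pickable, then stores the item's class on the character and destroys the actor.
; SnapToGround uses a short downward trace to set the item's height on BeginPlay and when the Bomb component's overlap ends.
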(event `self.PickupRadius.OnComponentBeginOverlap`
  (params (OverlappedComponent :type "PrimitiveComponent Object Reference") (OtherActor :type "Actor Object Reference") (OtherComp :type "PrimitiveComponent Object Reference") (OtherBodyIndex :type Integer) (bFromSweep :type Boolean) (SweepResult :type "HitResult Structure (by ref)"))
  ;[1 1 1] Item can be picked up when player overlaps
  (`/Engine/EditorBlueprintResources/StandardMacros.IsValid` (`self.CharacterREF`)
    (:`Is Valid`
      _)
    (:`Is Not Valid`
      (bind _asbp_third_person_character (cast `/Game/ThirdPerson/Blueprints/BP_ThirdPersonCharacter` OtherActor))
      (set `self.CharacterREF` _asbp_third_person_character)))
  (set `self.isPickable` true)
  (`KismetSystemLibrary.K2_SetTimerDelegate` (delegate `Pickup`) 0.1 true))

(event `Pickup`
  (bind _returnvalue (`GameplayStatics.GetObjectClass` self))
  ;[1 1 1] Item can be picked up when player overlaps
  ;;[1 1 1] Pickup Item
  (if (and (`/Game/ThirdPerson/Blueprints/BP_ThirdPersonCharacter.isInteracting` (`self.CharacterREF`)) (`self.isPickable`))
    (bind _output_get (set `/Game/ThirdPerson/Blueprints/BP_ThirdPersonCharacter.storedItem` _returnvalue (`self.CharacterREF`)))
    (if (== _output_get _returnvalue)
      (set `/Game/ThirdPerson/Blueprints/BP_ThirdPersonCharacter.holdingItem` true (`self.CharacterREF`))
      (`self.K2_DestroyActor`))))

(event `self.PickupRadius.OnComponentEndOverlap`
  (params (OverlappedComponent :type "PrimitiveComponent Object Reference") (OtherActor :type "Actor Object Reference") (OtherComp :type "PrimitiveComponent Object Reference") (OtherBodyIndex :type Integer))
  ;[1 1 1] Item can no longer be picked up
  (`/Engine/EditorBlueprintResources/StandardMacros.IsValid` (`self.CharacterREF`)
    (:`Is Valid`
      _)
    (:`Is Not Valid`
      (bind _asbp_third_person_character (cast `/Game/ThirdPerson/Blueprints/BP_ThirdPersonCharacter` OtherActor))
      (set `self.CharacterREF` _asbp_third_person_character)))
  (set `self.isPickable` false))

(event `self.ReceiveTick`
  (params (DeltaSeconds :type "Float (single-precision)"))
  ;[1 1 1] Debug
)

(event `self.ReceiveBeginPlay`
  (`self.Snap to Ground`))

(event `self.Bomb.OnComponentEndOverlap`
  (params (OverlappedComponent :type "PrimitiveComponent Object Reference") (OtherActor :type "Actor Object Reference") (OtherComp :type "PrimitiveComponent Object Reference") (OtherBodyIndex :type Integer))
  (`self.Snap to Ground`))

(fn `Snap to Ground`
  (bind _returnvalue (`self.K2_GetActorLocation`))
  (bind (_returnvalue_x _returnvalue_y) (`KismetMathLibrary.BreakVector` (`self.K2_GetActorLocation`)))
  (`self.SetActorHiddenInGame` true)
  (bind _outhit (`KismetSystemLibrary.LineTraceSingle` _returnvalue (+ _returnvalue (0.0 0.0 -200.0)) "TraceTypeQuery1"))
  (`self.K2_SetActorLocation` (`KismetMathLibrary.MakeVector` _returnvalue_x _returnvalue_y (.z (`.Location` (`GameplayStatics.BreakHitResult` _outhit)))))
  (`self.SetActorHiddenInGame` false))

(fn `UserConstructionScript`)