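; Door actor that opens and closes by sliding its Door component vertically.
; An OpenDoor event with an Interacted flag routes to open or close functions.
; Each function instantly sets the Door's world location to a fixed height offset above the scene root, higher for open and lower for closed, with no sweep or interpolation.
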(event `/Game/Assets/Blueprints/BI_Button.openDoor`
  (params (Interacted :type Boolean))
  (if Interacted
    (`self.doorOpen`)
    (else
      (`self.doorClose`))))

(fn `doorClose`
  (`SceneComponent.K2_SetWorldLocation` (`self.Door`) (+ (`SceneComponent.K2_GetComponentLocation` (`self.DefaultSceneRoot`)) (0.0 0.0 120.0)) false false))

(fn `doorOpen`
  (`SceneComponent.K2_SetWorldLocation` (`self.Door`) (+ (`SceneComponent.K2_GetComponentLocation` (`self.DefaultSceneRoot`)) (0.0 0.0 360.0)) false false))

(fn `UserConstructionScript`)