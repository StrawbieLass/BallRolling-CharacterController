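; BP_Item4 is a world item that the third-person character picks up by interacting inside its PickupRadius.
; Overlap caches the character and, if their hands are empty, marks the item pickable and starts a looping timer that polls for interact input; end overlap clears the flag.
; On pickup it stores its class on the character, sets HoldingItem and destroys itself.
; Once the character is cached, later overlaps skip the actor type check.
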(event `self.PickupRadius.OnComponentBeginOverlap`
  (params (OverlappedComponent :type "PrimitiveComponent Object Reference") (OtherActor :type "Actor Object Reference") (OtherComp :type "PrimitiveComponent Object Reference") (OtherBodyIndex :type Integer) (bFromSweep :type Boolean) (SweepResult :type "HitResult Structure (by ref)"))
  ;[1 1 1] Item can be picked up when player overlaps
  (`/Engine/EditorBlueprintResources/StandardMacros.IsValid` (`self.CharacterREF`)
    (:`Is Valid`
      _)
    (:`Is Not Valid`
      (bind _asbp_third_person_character (cast `/Game/ThirdPerson/Blueprints/BP_ThirdPersonCharacter` OtherActor))
      (bind _output_get (set `self.CharacterREF` _asbp_third_person_character))))
  (if (not (`/Game/ThirdPerson/Blueprints/BP_ThirdPersonCharacter.holdingItem` _output_get))
    (set `self.isPickable` true)
    (`KismetSystemLibrary.K2_SetTimerDelegate` (delegate `Pickup`) 0.1 true)))

(event `Pickup`
  (bind _returnvalue (`GameplayStatics.GetObjectClass` self))
  ;[1 1 1] Item can be picked up when player overlaps
  ;;[1 1 1] Pickup Item
  (if (and (`/Game/ThirdPerson/Blueprints/BP_ThirdPersonCharacter.isInteracting` (`self.CharacterREF`)) (`self.isPickable`))
    (bind _output_get (set `/Game/ThirdPerson/Blueprints/BP_ThirdPersonCharacter.storedItem` _returnvalue (`self.CharacterREF`)))
    (if (== _output_get _returnvalue)
      (set `/Game/ThirdPerson/Blueprints/BP_ThirdPersonCharacter.holdingItem` true (`self.CharacterREF`))
      (`self.K2_DestroyActor`))))

(event `self.PickupRadius.OnComponentEndOverlap`
  (params (OverlappedComponent :type "PrimitiveComponent Object Reference") (OtherActor :type "Actor Object Reference") (OtherComp :type "PrimitiveComponent Object Reference") (OtherBodyIndex :type Integer))
  ;[1 1 1] Item can no longer be picked up
  (`/Engine/EditorBlueprintResources/StandardMacros.IsValid` (`self.CharacterREF`)
    (:`Is Valid`
      _)
    (:`Is Not Valid`
      (bind _asbp_third_person_character (cast `/Game/ThirdPerson/Blueprints/BP_ThirdPersonCharacter` OtherActor))
      (set `self.CharacterREF` _asbp_third_person_character)))
  (set `self.isPickable` false))

(event `self.ReceiveTick`
  (params (DeltaSeconds :type "Float (single-precision)"))
  ;[1 1 1] Debug
)

(fn `UserConstructionScript`)