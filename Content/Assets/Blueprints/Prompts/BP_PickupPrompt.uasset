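; BP_PickupPrompt is an actor that shows a UI prompt while overlapped, hidden again on BeginPlay and when an overlap ends.
; PromptRadius overlap events toggle the UIPrompt component's visibility and the IsOverlapping flag.
; The first overlap must cast to BP_ThirdPersonCharacter, which is cached in CharacterREF.
; Once that reference is valid, any overlapping actor toggles the prompt without a further check.
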(event `self.PromptRadius.OnComponentBeginOverlap`
  (params (OverlappedComponent :type "PrimitiveComponent Object Reference") (OtherActor :type "Actor Object Reference") (OtherComp :type "PrimitiveComponent Object Reference") (OtherBodyIndex :type Integer) (bFromSweep :type Boolean) (SweepResult :type "HitResult Structure (by ref)"))
  (`/Engine/EditorBlueprintResources/StandardMacros.IsValid` (`self.CharacterREF`)
    (:`Is Valid`
      _)
    (:`Is Not Valid`
      (bind _asbp_third_person_character (cast `/Game/ThirdPerson/Blueprints/BP_ThirdPersonCharacter` OtherActor))
      (set `self.CharacterREF` _asbp_third_person_character)))
  (set `self.isOverlapping` true)
  (`SceneComponent.SetVisibility` (`self.UIPrompt`) true false))

(event `self.PromptRadius.OnComponentEndOverlap`
  (params (OverlappedComponent :type "PrimitiveComponent Object Reference") (OtherActor :type "Actor Object Reference") (OtherComp :type "PrimitiveComponent Object Reference") (OtherBodyIndex :type Integer))
  (`/Engine/EditorBlueprintResources/StandardMacros.IsValid` (`self.CharacterREF`)
    (:`Is Valid`
      _)
    (:`Is Not Valid`
      (bind _asbp_third_person_character (cast `/Game/ThirdPerson/Blueprints/BP_ThirdPersonCharacter` OtherActor))
      (set `self.CharacterREF` _asbp_third_person_character)))
  (set `self.isOverlapping` false)
  (`SceneComponent.SetVisibility` (`self.UIPrompt`) false false))

(event `self.ReceiveBeginPlay`
  (`SceneComponent.SetVisibility` (`self.UIPrompt`) false false))

(fn `UserConstructionScript`)