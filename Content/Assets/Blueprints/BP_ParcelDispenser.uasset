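; Parcel dispenser actor that spawns a BP_Item5 at its own transform on BeginPlay and replaces it when it is gone.
; A looping 5-second timer checks whether the stored box reference is still valid and whether the player's StoredItem is BP_Item5.
; If the box is gone and the player is not holding one, it spawns and tracks a new one after a delay.
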(event `self.ReceiveBeginPlay`
  (bind _returnvalue (`self.SpawnBox`))
  (set `self.BoxREF` _returnvalue)
  (`KismetSystemLibrary.K2_SetTimerDelegate` (delegate `Respawn on Destroyed`) 5.0 true))

(event `Respawn on Destroyed`
  (`/Engine/EditorBlueprintResources/StandardMacros.IsValid` (`self.BoxREF`)
    (:`Is Not Valid`
      (bind _return_value (`self.playerHasBox?`))
      (if (not _return_value)
        (`KismetSystemLibrary.Delay` 10.0)
        (bind _returnvalue (`self.SpawnBox`))
        (set `self.BoxREF` _returnvalue)))))

(fn `playerHasBox?`
  (returns (`Return Value` :type Boolean))
  (bind _asbp_third_person_character (cast `/Game/ThirdPerson/Blueprints/BP_ThirdPersonCharacter` (`GameplayStatics.GetPlayerPawn` 0)))
  (return (== (`/Game/ThirdPerson/Blueprints/BP_ThirdPersonCharacter.storedItem` _asbp_third_person_character) "/Game/Assets/Blueprints/Items/BP_Item5.BP_Item5_C")))

(fn `SpawnBox`
  (returns (ReturnValue :type "/Game/Assets/Blueprints/Items/BP_Item5 Object Reference"))
  (bind _returnvalue (`|SpawnActorFromClass` "/Game/Assets/Blueprints/Items/BP_Item5.BP_Item5_C" (`self.GetTransform`) "Undefined" "MultiplyWithRoot" null null))
  (return _returnvalue))

(fn `UserConstructionScript`)