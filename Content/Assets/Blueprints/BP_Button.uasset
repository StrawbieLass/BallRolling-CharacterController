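; BP_Button is a pressure button that opens and closes a linked Gate when an actor tagged "Buttonable" enters or leaves its sphere.
; Both overlap events call ButtonToggle, which snaps the Button component down or back up and passes the state to the Gate through an OpenDoor message.
; A DoOnce guards the press and resets shortly after any tagged actor exits.
; ButtonPress and ButtonReset are unused stubs.
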(event `self.Sphere.OnComponentBeginOverlap`
  (params (OverlappedComponent :type "PrimitiveComponent Object Reference") (OtherActor :type "Actor Object Reference") (OtherComp :type "PrimitiveComponent Object Reference") (OtherBodyIndex :type Integer) (bFromSweep :type Boolean) (SweepResult :type "HitResult Structure (by ref)"))
  (bind _returnvalue (`self.ActorHasTag` OtherActor "Buttonable"))
  (if _returnvalue
    (`/Engine/EditorBlueprintResources/StandardMacros.DoOnce` false :!label _label
      (:`Completed`
        (`self.Button Toggle` _returnvalue)))))

(event `self.Sphere.OnComponentEndOverlap`
  (params (OverlappedComponent :type "PrimitiveComponent Object Reference") (OtherActor :type "Actor Object Reference") (OtherComp :type "PrimitiveComponent Object Reference") (OtherBodyIndex :type Integer))
  (if (`self.ActorHasTag` OtherActor "Buttonable")
    (`self.Button Toggle` false)
    (`KismetSystemLibrary.Delay` 0.02)
    (goto _label :!via `Reset`)))

(event `Button Toggle`
  (params (Triggered :type Boolean))
  ;[1 1 1] fancy stuff
  (`SceneComponent.K2_SetRelativeLocation` (`self.Button`) (`KismetMathLibrary.SelectVector` (0.0 0.0 -10.0) (0.0 0.0 0.0) Triggered) false false)
  (message `/Game/Assets/Blueprints/BI_Button.openDoor` (`self.Gate`) Triggered))

(fn `ButtonPress`)

(fn `ButtonReset`)

(fn `UserConstructionScript`)