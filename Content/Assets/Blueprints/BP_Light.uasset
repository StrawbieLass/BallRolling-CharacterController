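; BP_Light is an indicator light actor that reflects a door's open or closed state.
; The OpenDoor event swaps the Light component's material to green or red depending on its Interacted flag.
; Separate DoorOpen and DoorClose functions snap the Light to a higher or lower vertical offset from the scene root, without sweeping, and are not called within this Blueprint.
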(event `self.openDoor`
  (params (Interacted :type Boolean))
  (bind _light (`self.Light`))
  (if Interacted
    (`PrimitiveComponent.SetMaterial` _light 0 "/Game/Assets/Materials/M_GreenLight.M_GreenLight")
    (else
      (`PrimitiveComponent.SetMaterial` _light 0 "/Game/Assets/Materials/M_RedLight.M_RedLight"))))

(fn `doorClose`
  (`SceneComponent.K2_SetWorldLocation` (`self.Light`) (+ (`SceneComponent.K2_GetComponentLocation` (`self.DefaultSceneRoot`)) (0.0 0.0 120.0)) false false))

(fn `doorOpen`
  (`SceneComponent.K2_SetWorldLocation` (`self.Light`) (+ (`SceneComponent.K2_GetComponentLocation` (`self.DefaultSceneRoot`)) (0.0 0.0 360.0)) false false))

(fn `UserConstructionScript`)